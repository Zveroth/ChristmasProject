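; Player pawn that creates the player UI, moves by axis input, interacts with overlapped actors on E and can spawn a stolen gift.
; Tick applies swept movement, turns the mesh and, on blocking hits, adds a second offset angled from the impact normal.
; Shift sprinting drains a stamina pool that regenerates after a release delay, both updating only while moving.
; A wall capsule fades overlapped transparent blocks out and back in.
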(event `self.ReceiveBeginPlay`
  (bind _wallcapsule (`self.WallCapsule`))
  (add `PrimitiveComponent.OnComponentBeginOverlap` _wallcapsule (delegate `WallBeginOverlap`))
  (add `PrimitiveComponent.OnComponentEndOverlap` _wallcapsule (delegate `WallEndOverlap`))
  (bind _returnvalue (`|CreateWidget` "/Game/UI/BP_PlayerUI.BP_PlayerUI_C" (`GameplayStatics.GetPlayerController` 0)))
  (`UserWidget.AddToViewport` _returnvalue 0))

(event `WallBeginOverlap`
  (params (OverlappedComponent :type "PrimitiveComponent Object Reference") (OtherActor :type "Actor Object Reference") (OtherComp :type "PrimitiveComponent Object Reference") (OtherBodyIndex :type Integer) (bFromSweep :type Boolean) (SweepResult :type "HitResult Structure (by ref)"))
  (bind _asbp_transparent_block (cast `/Game/Blueprints/Level/BP_TransparentBlock` OtherActor))
  (`/Game/Blueprints/Level/BP_TransparentBlock.FadeOut` _asbp_transparent_block))

(event `WallEndOverlap`
  (params (OverlappedComponent :type "PrimitiveComponent Object Reference") (OtherActor :type "Actor Object Reference") (OtherComp :type "PrimitiveComponent Object Reference") (OtherBodyIndex :type Integer))
  (bind _asbp_transparent_block (cast `/Game/Blueprints/Level/BP_TransparentBlock` OtherActor))
  (`/Game/Blueprints/Level/BP_TransparentBlock.FadeIn` _asbp_transparent_block))

(event `self.ReceiveTick`
  (params (DeltaSeconds :type "Float (single-precision)"))
  (bind _movementdir (`self.MovementDir`))
  (bind _returnvalue (`KismetMathLibrary.Conv_VectorToRotator` (`self.MovementDir`)))
  (bind _returnvalue_2 (`KismetMathLibrary.Normal` _movementdir))
  ;[1 1 1] Move the player
  (if (`self.bUsingShortcut`)
    _
    (elif (!= _movementdir (`KismetMathLibrary.Vector_Zero`) :`ErrorTolerance` 0.001)
      (if (`self.bSprinting`)
        (bind _output_get (set `self.SprintLeft` (- (`self.SprintLeft`) DeltaSeconds)))
        (if (<= _output_get 0.0)
          (set `self.MovementSpeed` 300.0)
          (set `self.SprintLeft` 0.0))
        (elif (`self.bCanRegenSprint`)
          (bind _output_get_2 (set `self.SprintLeft` (+ (`self.SprintLeft`) (* DeltaSeconds 0.7))))
          (if (> _output_get_2 3.0)
            (set `self.SprintLeft` 3.0))))
      (`SceneComponent.K2_SetWorldRotation` (`self.PlayerMesh`) (`KismetMathLibrary.Conv_VectorToRotator` _returnvalue_2) false false)
      (bind _sweephitresult (`self.K2_AddActorWorldOffset` (* (* _returnvalue_2 DeltaSeconds) (`self.MovementSpeed`)) true))
      (bind (_bblockinghit _binitialoverlap _time _distance _location _impactpoint _normal _impactnormal) (`GameplayStatics.BreakHitResult` _sweephitresult))
      ;[1 1 1] Handle blocking walls
      (if _bblockinghit
        (bind _returnvalue_3 (- (- (.yaw _returnvalue) (.yaw (`KismetMathLibrary.Conv_VectorToRotator` _impactnormal))) 180.0))
        (if (< _returnvalue_3 -180.0)
          (`self.K2_AddActorWorldOffset` (* (`KismetMathLibrary.Conv_RotatorToVector` (`KismetMathLibrary.ComposeRotators` _returnvalue (`KismetMathLibrary.MakeRotator` 0.0 0.0 (+ 360.0 _returnvalue_3)))) (* (`self.MovementSpeed`) DeltaSeconds)) true)
          (elif (> _returnvalue_3 180.0)
            (`self.K2_AddActorWorldOffset` (* (`KismetMathLibrary.Conv_RotatorToVector` (`KismetMathLibrary.ComposeRotators` _returnvalue (`KismetMathLibrary.MakeRotator` 0.0 0.0 (+ -360.0 _returnvalue_3)))) (* (`self.MovementSpeed`) DeltaSeconds)) true)
            (else
              (`self.K2_AddActorWorldOffset` (* (`KismetMathLibrary.Conv_RotatorToVector` (`KismetMathLibrary.ComposeRotators` _returnvalue (`KismetMathLibrary.MakeRotator` 0.0 0.0 _returnvalue_3))) (* (`self.MovementSpeed`) DeltaSeconds)) true))))))))

(event `InputAxis|MoveX`
  (params (AxisValue :type "Float (single-precision)"))
  (set `self.MovementDir` (`KismetMathLibrary.MakeVector` AxisValue (.y (`self.MovementDir`)))))

(event `InputAxis|MoveY`
  (params (AxisValue :type "Float (single-precision)"))
  (set `self.MovementDir` (`KismetMathLibrary.MakeVector` (.x (`self.MovementDir`)) AxisValue)))

(event `Key|E`
  (params (Key :type "Key Structure"))
  (:`Pressed`
    (if (not (`self.bUsingShortcut`))
      (for _array_element (`PrimitiveComponent.GetOverlappingActors` (`self.InteractionCapsule`) null)
        (bind _bsuccess (message `/Game/Blueprints/Misc/BP_Interactable.Interact` _array_element))
        (if _bsuccess
          (break))))))

(event `Key|LeftShift`
  (params (Key :type "Key Structure"))
  (:`Pressed`
    (set `self.bSprinting` true)
    (set `self.MovementSpeed` 500.0)
    (set `self.bCanRegenSprint` false))
  (:`Released`
    (set `self.bSprinting` false)
    (set `self.MovementSpeed` 300.0)
    (`KismetSystemLibrary.K2_ClearAndInvalidateTimerHandle` (`self.SprintTimer`))
    (bind _returnvalue (`KismetSystemLibrary.K2_SetTimerDelegate` (delegate `CustomEvent_0`) 1.0))
    (set `self.SprintTimer` _returnvalue)))

(event `CustomEvent_0`
  (set `self.bCanRegenSprint` true))

(fn `GetPlayerForwardVector`
  (returns (Direction :type "Vector Structure"))
  (return (`SceneComponent.GetForwardVector` (`self.PlayerMesh`))))

(fn `TakeGift`
  (bind _direction (`self.GetPlayerForwardVector`))
  (`|SpawnActorFromClass` "/Game/Blueprints/Misc/BP_StolenGift.BP_StolenGift_C" (`KismetMathLibrary.MakeTransform` (+ (`self.K2_GetActorLocation`) (* _direction 15.0)) (`KismetMathLibrary.Conv_VectorToRotator` _direction)) "AlwaysSpawn" "OverrideRootScale" null null))

(fn `UserConstructionScript`)