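; Bear trap that the player carries and places to trap Santa.
; While not placed, it follows just ahead of the player every Tick; Interact toggles between dropping it lower and picking it back up.
; Overlap events on SantaDet set an in-range flag; when placed, Tick calls TrapSanta on the first overlapping actor, cast to BP_Santa.
; Triggering spawns an activation emitter, blocks further interaction and destroys the trap after a delay.
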(event `self.ReceiveBeginPlay`
  (bind _santadet (`self.SantaDet`))
  (add `PrimitiveComponent.OnComponentBeginOverlap` _santadet (delegate `OnComponentBeginOverlap_Event_0`))
  (add `PrimitiveComponent.OnComponentEndOverlap` _santadet (delegate `OnComponentEndOverlap_Event_0`))
  (set `self.PlayerRef` (cast `/Game/Blueprints/Player/BP_PlayerPawn` (`GameplayStatics.GetPlayerPawn` 0) :!pure true)))

(event `OnComponentBeginOverlap_Event_0`
  (params (OverlappedComponent :type "PrimitiveComponent Object Reference") (OtherActor :type "Actor Object Reference") (OtherComp :type "PrimitiveComponent Object Reference") (OtherBodyIndex :type Integer) (bFromSweep :type Boolean) (SweepResult :type "HitResult Structure (by ref)"))
  (set `self.bSantaInRange` true))

(event `OnComponentEndOverlap_Event_0`
  (params (OverlappedComponent :type "PrimitiveComponent Object Reference") (OtherActor :type "Actor Object Reference") (OtherComp :type "PrimitiveComponent Object Reference") (OtherBodyIndex :type Integer))
  (set `self.bSantaInRange` false))

(event `self.ReceiveTick`
  (params (DeltaSeconds :type "Float (single-precision)"))
  (bind _playerref (`self.PlayerRef`))
  (if (`self.bUsedUp`)
    _
    (elif (`self.bPlacedDown`)
      (if (`self.bSantaInRange`)
        (`/Game/Blueprints/Santa/BP_Santa.TrapSanta` (cast `/Game/Blueprints/Santa/BP_Santa` (`|GetArrayItem` (`PrimitiveComponent.GetOverlappingActors` (`self.SantaDet`) null)) :!pure true))
        (set `self.bUsedUp` true)
        (`GameplayStatics.SpawnEmitterAtLocation` "/Game/Particles/BearTrap_Activate.BearTrap_Activate" (`self.K2_GetActorLocation`))
        (`KismetSystemLibrary.K2_SetTimerDelegate` (delegate `CustomEvent_0`) 10.0))
      (else
        (bind _direction (`/Game/Blueprints/Player/BP_PlayerPawn.GetPlayerForwardVector` _playerref))
        (`self.K2_SetActorLocation` (+ (* _direction 15.0) (`self.K2_GetActorLocation` _playerref)))))))

(event `CustomEvent_0`
  (`self.K2_DestroyActor`))

(fn `Interact`
  (returns (bSuccess :type Boolean))
  (if (`self.bUsedUp`)
    (return false)
    (else
      (if (`self.bPlacedDown`)
        (set `self.bPlacedDown` false)
        (else
          (`self.K2_AddActorLocalOffset` (0.0 0.0 -50.0))
          (set `self.bPlacedDown` true)))
      (return true))))

(fn `UserConstructionScript`)