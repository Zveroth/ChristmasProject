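; BP_Doors is a level door actor that swings open once, in a single instant step with no animation.
; OpenDoors checks the Opened flag and returns false if set; otherwise it shifts and rotates the actor, sets the flag and returns true.
; The shift feeds world-space forward and right vectors into a local-space offset, without sweep.
; The event graph holds only disabled stubs, so opening relies on an external call.
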(fn `OpenDoors`
  (returns (Successful :type Boolean))
  (if (`self.bOpened`)
    (return false)
    (else
      (`self.K2_AddActorLocalOffset` (+ (* (`self.GetActorForwardVector`) -65.0) (* (`self.GetActorRightVector`) 10.0)))
      (set `self.bOpened` true)
      (`self.K2_AddActorWorldRotation` (struct :`Yaw` 160.0))
      (return true))))

(fn `UserConstructionScript`)