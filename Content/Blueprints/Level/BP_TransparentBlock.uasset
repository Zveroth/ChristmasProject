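; BP_TransparentBlock is a level block whose wall mesh fades between full opacity and a minimum opacity.
; BeginPlay creates a dynamic material instance for the wall mesh.
; FadeIn and FadeOut set the fade direction, enable Tick and print a debug string.
; Tick moves the WallOpacity material parameter in that direction and disables itself once the limit is reached.
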(event `self.ReceiveBeginPlay`
  (bind _wallmesh (`self.WallMesh`))
  (bind _returnvalue (`KismetMaterialLibrary.CreateDynamicMaterialInstance` (`PrimitiveComponent.GetMaterial` _wallmesh 0)))
  (bind _output_get (set `self.WallMat` _returnvalue))
  (`PrimitiveComponent.SetMaterial` _wallmesh 0 _output_get))

(event `self.ReceiveTick`
  (params (DeltaSeconds :type "Float (single-precision)"))
  (bind _opacitychange (`self.OpacityChange`))
  (bind _minimumopacity (`self.MinimumOpacity`))
  (set `self.CurrentOpacity` (+ (`self.CurrentOpacity`) (* DeltaSeconds _opacitychange 2.0)))
  (if (== _opacitychange 1.0)
    (if (>= (`self.CurrentOpacity`) 1.0)
      (set `self.CurrentOpacity` 1.0)
      (`self.SetActorTickEnabled` false))
    (elif (<= (`self.CurrentOpacity`) _minimumopacity)
      (set `self.CurrentOpacity` _minimumopacity)
      (`self.SetActorTickEnabled` false)))
  (`MaterialInstanceDynamic.SetScalarParameterValue` (`self.WallMat`) "WallOpacity" (`self.CurrentOpacity`)))

(fn `FadeIn`
  (`self.SetActorTickEnabled` true)
  (set `self.OpacityChange` 1.0)
  (`KismetSystemLibrary.PrintString` "In "))

(fn `FadeOut`
  (`self.SetActorTickEnabled` true)
  (set `self.OpacityChange` -1.0)
  (`KismetSystemLibrary.PrintString` "Out"))

(fn `UserConstructionScript`)