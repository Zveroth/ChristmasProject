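; BP_Keys is a key actor the player can pick up, carry and use on doors.
; Interact picks it up, and Tick then holds it just ahead of the player pawn along its forward vector.
; Interacting while held calls OpenDoors on BP_Doors overlapping the capsule, destroying the key on success.
; The key drops downward only when nothing overlaps the capsule.
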(event `self.ReceiveBeginPlay`
  (set `self.PlayerRef` (cast `/Game/Blueprints/Player/BP_PlayerPawn` (`GameplayStatics.GetPlayerPawn` 0) :!pure true)))

(event `self.ReceiveTick`
  (params (DeltaSeconds :type "Float (single-precision)"))
  (bind _playerref (`self.PlayerRef`))
  (if (`self.bPickedUp`)
    (bind _direction (`/Game/Blueprints/Player/BP_PlayerPawn.GetPlayerForwardVector` _playerref))
    (`self.K2_SetActorLocation` (+ (* _direction 15.0) (`self.K2_GetActorLocation` _playerref)))))

(fn `Interact`
  (returns (bSuccess :type Boolean))
  (bind _overlappingactors (`PrimitiveComponent.GetOverlappingActors` (`self.Capsule`) null))
  (if (`self.bPickedUp`)
    (if (> (`KismetArrayLibrary.Array_Length` _overlappingactors) 0)
      (for _array_element _overlappingactors
        (bind _asbp_doors (cast `/Game/Blueprints/Level/BP_Doors` _array_element))
        (bind _successful (`/Game/Blueprints/Level/BP_Doors.OpenDoors` _asbp_doors))
        (if _successful
          (`self.K2_DestroyActor`)
          (return true)))
      (return true)
      (else
        (`self.K2_AddActorLocalOffset` (0.0 0.0 -35.0))
        (set `self.bPickedUp` false)
        (return true)))
    (else
      (set `self.bPickedUp` true)
      (return true))))

(fn `UserConstructionScript`)