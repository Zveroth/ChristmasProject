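; Level shortcut actor that carries the player between its two endpoints, PointA and PointB, in either direction.
; UseShortcut disables input, flags the player as using a shortcut, snaps them to the nearer endpoint and enables Tick.
; Tick moves the player straight to the opposite point without sweeping, at MovementSpeed scaled by MovementMultiplier.
; On arrival it snaps to the point, restores input and turns Tick off.
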(event `self.ReceiveBeginPlay`
  (set `self.PlayerRef` (cast `/Game/Blueprints/Player/BP_PlayerPawn` (`GameplayStatics.GetPlayerPawn` 0) :!pure true)))

(event `self.ReceiveTick`
  (params (DeltaSeconds :type "Float (single-precision)"))
  (bind _playerref (`self.PlayerRef`))
  (bind _playerref_2 (`self.PlayerRef`))
  (bind _playerref_3 (`self.PlayerRef`))
  (bind _playerref_4 (`self.PlayerRef`))
  (bind _returnvalue (`SceneComponent.K2_GetComponentLocation` (`self.PointB`)))
  (bind _returnvalue_2 (`SceneComponent.K2_GetComponentLocation` (`self.PointA`)))
  (bind _returnvalue_3 (- _returnvalue (`self.K2_GetActorLocation` _playerref_3)))
  (bind _returnvalue_4 (- _returnvalue_2 (`self.K2_GetActorLocation` _playerref)))
  (bind _returnvalue_5 (* (`/Game/Blueprints/Player/BP_PlayerPawn.MovementSpeed` _playerref) DeltaSeconds (`self.MovementMultiplier`)))
  (bind _returnvalue_6 (* (`/Game/Blueprints/Player/BP_PlayerPawn.MovementSpeed` _playerref_3) DeltaSeconds (`self.MovementMultiplier`)))
  (if (`self.AtoB`)
    (if (<= (`KismetMathLibrary.VSize` _returnvalue_3) _returnvalue_6)
      (`self.K2_SetActorLocation` _playerref_4 _returnvalue false false)
      (set `/Game/Blueprints/Player/BP_PlayerPawn.bUsingShortcut` false _playerref_4)
      (`self.EnableInput` _playerref_4 null)
      (`self.SetActorTickEnabled` false)
      (else
        (`self.K2_AddActorWorldOffset` _playerref_4 (* (`KismetMathLibrary.Normal` _returnvalue_3) _returnvalue_6) false false)))
    (elif (<= (`KismetMathLibrary.VSize` _returnvalue_4) _returnvalue_5)
      (`self.K2_SetActorLocation` _playerref_2 _returnvalue_2 false false)
      (set `/Game/Blueprints/Player/BP_PlayerPawn.bUsingShortcut` false _playerref_2)
      (`self.EnableInput` _playerref_2 null)
      (`self.SetActorTickEnabled` false)
      (else
        (`self.K2_AddActorWorldOffset` _playerref_2 (* (`KismetMathLibrary.Normal` _returnvalue_4) _returnvalue_5) false false)))))

(fn `UserConstructionScript`)

(fn `UseShortcut`
  (bind _playerref (`self.PlayerRef`))
  (bind _returnvalue (`self.K2_GetActorLocation` _playerref))
  (bind _returnvalue_2 (`SceneComponent.K2_GetComponentLocation` (`self.PointB`)))
  (bind _returnvalue_3 (`SceneComponent.K2_GetComponentLocation` (`self.PointA`)))
  (bind _returnvalue_4 (- _returnvalue_2 _returnvalue))
  (bind _returnvalue_5 (- _returnvalue_3 _returnvalue))
  (`self.DisableInput` _playerref null)
  (set `/Game/Blueprints/Player/BP_PlayerPawn.bUsingShortcut` true _playerref)
  (`self.SetActorTickEnabled` true)
  (if (< (`KismetMathLibrary.VSize` _returnvalue_5) (`KismetMathLibrary.VSize` _returnvalue_4))
    (set `self.AtoB` true)
    (`self.K2_SetActorLocation` _playerref _returnvalue_3 false false)
    (`SceneComponent.K2_SetWorldRotation` (`/Game/Blueprints/Player/BP_PlayerPawn.PlayerMesh` _playerref) (`KismetMathLibrary.Conv_VectorToRotator` _returnvalue_5) false false)
    (else
      (set `self.AtoB` false)
      (`self.K2_SetActorLocation` _playerref _returnvalue_2 false false)
      (`SceneComponent.K2_SetWorldRotation` (`/Game/Blueprints/Player/BP_PlayerPawn.PlayerMesh` _playerref) (`KismetMathLibrary.Conv_VectorToRotator` _returnvalue_4) false false))))