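; BP_Santa is the AI-driven Santa character, which starts invisible and can hide at hide spots.
; Any box collision overlap freezes its movement for TrapDuration, then restores walk speed.
; When the overlap is a BP_SantaHideSpot, a percentage roll can write the spot's location and a want-to-hide flag to the AI controller's blackboard.
; SantaHiding records the hidden state and toggles capsule visibility, while Interact simply returns false.
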(event `self.ReceiveBeginPlay`
  (`self.SetActive` false))

(event `self.BoxCollition.OnComponentBeginOverlap`
  (params (OverlappedComponent :type "PrimitiveComponent Object Reference") (OtherActor :type "Actor Object Reference") (OtherComp :type "PrimitiveComponent Object Reference") (OtherBodyIndex :type Integer) (bFromSweep :type Boolean) (SweepResult :type "HitResult Structure (by ref)"))
  (`self.TrapSanta`)
  (bind _asbp_santa_hide_spot (cast `/Game/Blueprints/BP_SantaHideSpot` OtherActor))
  (if (<= (`KismetMathLibrary.RandomFloatInRange` 0.0 100.0) (`self.fHidePercentage`))
    (bind _assanta_aicontroller (cast `/Game/Blueprints/Santa/Santa_AIController` (`AIBlueprintHelperLibrary.GetAIController` self))
      (:`then`
        (bind _returnvalue (`AIBlueprintHelperLibrary.GetBlackboard` _assanta_aicontroller))
        (`BlackboardComponent.SetValueAsVector` _returnvalue "HideLocation" (`self.K2_GetActorLocation` _asbp_santa_hide_spot))
        (`BlackboardComponent.SetValueAsBool` _returnvalue "bIsSantaWantToHide" true))
      (:`CastFailed`
        (`BlackboardComponent.SetValueAsBool` _returnvalue "bIsSantaWantToHide" false)))))

(event `TrapSanta`
  (bind _charactermovement (`self.CharacterMovement`))
  (set `CharacterMovementComponent.MaxWalkSpeed` 0.0 _charactermovement)
  (`KismetSystemLibrary.Delay` (`self.TrapDuration`))
  (set `CharacterMovementComponent.MaxWalkSpeed` 600.0 _charactermovement))

(fn `Interact`
  (returns (bSuccess :type Boolean))
  (return false))

(fn `SantaHiding`
  (params (NewValue :type Boolean))
  (set `self.bIsSantaHide` NewValue)
  (`SceneComponent.SetVisibility` (`self.CapsuleComponent`) (not NewValue) true))

(fn `SetActive`
  (params (NewValue :type Boolean))
  (`SceneComponent.SetVisibility` (`self.CapsuleComponent`) NewValue true))

(fn `UserConstructionScript`)