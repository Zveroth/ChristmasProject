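; Behavior tree task that spawns Santa into play at his blackboard spawn location.
; It teleports the controlled pawn to a random navigable point within a small radius of SpawnLocation.
; It then activates BP_Santa, sets bSantaIsSpawned, clears bisTheGivePlaced and finishes successfully.
; A failed cast to BP_Santa stops the task before it calls FinishExecute.
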(event `self.ReceiveExecuteAI`
  (params (OwnerController :type "AIController Object Reference") (ControlledPawn :type "Pawn Object Reference"))
  (bind _returnvalue (`AIBlueprintHelperLibrary.GetBlackboard` OwnerController))
  (bind _randomlocation (`NavigationSystemV1.K2_GetRandomLocationInNavigableRadius` (`BlackboardComponent.GetValueAsVector` _returnvalue "SpawnLocation") 50.0 null null))
  (`Actor.K2_SetActorLocation` ControlledPawn _randomlocation false true)
  (bind _asbp_santa (cast `/Game/Blueprints/Santa/BP_Santa` ControlledPawn))
  (`/Game/Blueprints/Santa/BP_Santa.SetActive` _asbp_santa true)
  (`BlackboardComponent.SetValueAsBool` _returnvalue "bSantaIsSpawned" true)
  (`BlackboardComponent.SetValueAsBool` _returnvalue "bisTheGivePlaced" false)
  (`self.FinishExecute` true))