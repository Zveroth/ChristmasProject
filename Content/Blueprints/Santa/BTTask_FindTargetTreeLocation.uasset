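; Behavior tree task for the Santa AI that picks a random tree target still awaiting a present.
; On execute it shuffles all BP_TreeTarget actors and loops over them, though each pass tests only the first element's PresentSent flag.
; If that tree is unserved, it breaks, writes the tree's location and object to the Blackboard and finishes successfully.
; Otherwise the task never calls FinishExecute.
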(event `self.ReceiveExecuteAI`
  (params (OwnerController :type "AIController Object Reference") (ControlledPawn :type "Pawn Object Reference"))
  (bind _returnvalue (`AIBlueprintHelperLibrary.GetBlackboard` OwnerController))
  (bind _outactors (`GameplayStatics.GetAllActorsOfClass` "/Game/Blueprints/BP_TreeTarget.BP_TreeTarget_C"))
  (`KismetArrayLibrary.Array_Shuffle` _outactors)
  (for _ _outactors
    (bind _output (`|GetArrayItem` _outactors))
    (if (not (`/Game/Blueprints/BP_TreeTarget.PresentSent` _output))
      (`|ExecutionSequence`
        (:`then_0`
          (break))
        (:`then_1`
          (`BlackboardComponent.SetValueAsVector` _returnvalue "TreeTargetLocation" (`Actor.K2_GetActorLocation` _output))
          (`BlackboardComponent.SetValueAsObject` _returnvalue "TreeTargetObject" _output)
          (`self.FinishExecute` true))))))