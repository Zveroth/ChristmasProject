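; Santa_AIController is the AI controller for the Santa character, running the BT_Santa behavior tree on BeginPlay.
; AI perception updates that involve the player pawn set the bIsSeeplayer blackboard key and switch Santa to his see-player walk speed.
; Updates that involve a hide spot pass it to Santa's SantaThinkToHide.
; The handler ignores whether the stimulus was gained or lost, so it never clears the flag.
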(event `self.ReceiveBeginPlay`
  (`self.RunBehaviorTree` "/Game/Blueprints/Santa/BT_Santa.BT_Santa"))

(event `self.AIPerception.OnTargetPerceptionUpdated`
  (params (Actor :type "Actor Object Reference") (Stimulus :type "AIStimulus Structure"))
  (`|ExecutionSequence`
    (:`then_0`
      (cast `/Game/Blueprints/Player/BP_PlayerPawn` Actor)
      (`KismetSystemLibrary.PrintString` "SeePlayer")
      (`BlackboardComponent.SetValueAsBool` (`AIBlueprintHelperLibrary.GetBlackboard` null) "bIsSeeplayer" true)
      (bind _asbp_santa (cast `/Game/Blueprints/Santa/BP_Santa` (`self.K2_GetPawn`)))
      (set `CharacterMovementComponent.MaxWalkSpeed` (`/Game/Blueprints/Santa/BP_Santa.SeePlayerWalkSpeed` _asbp_santa) (`Character.CharacterMovement` _asbp_santa)))
    (:`then_1`
      (bind _asbp_santa_hide_spot (cast `/Game/Blueprints/BP_SantaHideSpot` Actor))
      (bind _asbp_santa_2 (cast `/Game/Blueprints/Santa/BP_Santa` (`self.K2_GetPawn`)))
      (`/Game/Blueprints/Santa/BP_Santa.SantaThinkToHide` _asbp_santa_2 _asbp_santa_hide_spot))))

(fn `UserConstructionScript`)