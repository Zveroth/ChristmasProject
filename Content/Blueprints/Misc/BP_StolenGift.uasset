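; BP_StolenGift is a gift the player carries and delivers for a point.
; Interact toggles carrying; while carried, Tick keeps the gift just ahead of the player, facing the same way.
; Dropping offsets it downward, and any actor overlapping its Capsule counts as the goal.
; Delivery plays a particle effect, increments the player's Points, stops Tick and blocks further pickup.
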(event `self.ReceiveBeginPlay`
  (set `self.PlayerRef` (cast `/Game/Blueprints/Player/BP_PlayerPawn` (`GameplayStatics.GetPlayerPawn` 0) :!pure true)))

(event `self.ReceiveTick`
  (params (DeltaSeconds :type "Float (single-precision)"))
  (bind _playerref (`self.PlayerRef`))
  (if (`self.bPickedUp`)
    (bind _direction (`/Game/Blueprints/Player/BP_PlayerPawn.GetPlayerForwardVector` _playerref))
    (`self.K2_SetActorLocation` (+ (* _direction 15.0) (`self.K2_GetActorLocation` _playerref)))
    (`self.K2_SetActorRotation` (`KismetMathLibrary.Conv_VectorToRotator` _direction))))

(fn `Interact`
  (returns (bSuccess :type Boolean))
  (if (`self.bPickedUp`)
    (set `self.bPickedUp` false)
    (`self.K2_AddActorLocalOffset` (0.0 0.0 -50.0))
    (if (> (`KismetArrayLibrary.Array_Length` (`PrimitiveComponent.GetOverlappingActors` (`self.Capsule`) null)) 0)
      (set `self.bAtGoal` true)
      (`self.SetActorTickEnabled` false)
      (`GameplayStatics.SpawnEmitterAtLocation` "/Game/Particles/PresentDelivered.PresentDelivered" (`self.K2_GetActorLocation`))
      (`/Engine/EditorBlueprintResources/StandardMacros.IncrementInt` (`/Game/Blueprints/Player/BP_PlayerPawn.Points` (`self.PlayerRef`))
        (:`  `
          (return true)))
      (else
        (return true)))
    (elif (`self.bAtGoal`)
      (return false)
      (else
        (set `self.bPickedUp` true)
        (return true)))))

(fn `UserConstructionScript`)