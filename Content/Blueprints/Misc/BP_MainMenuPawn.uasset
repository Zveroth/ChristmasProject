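; BP_MainMenuPawn is the pawn behind the main menu, providing a gently swaying camera view.
; On BeginPlay it creates the BP_MainMenu widget for the first player controller and adds it to the viewport.
; Each Tick advances an angle accumulator and feeds its sine into the Camera's relative yaw, panning side to side at a fixed slight downward pitch.
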(event `self.ReceiveBeginPlay`
  (bind _returnvalue (`|CreateWidget` "/Game/UI/BP_MainMenu.BP_MainMenu_C" (`GameplayStatics.GetPlayerController` 0)))
  (`UserWidget.AddToViewport` _returnvalue 0))

(event `self.ReceiveTick`
  (params (DeltaSeconds :type "Float (single-precision)"))
  (bind _output_get (set `self.A` (+ (`self.A`) (* DeltaSeconds 25.0))))
  (`SceneComponent.K2_SetRelativeRotation` (`self.Camera`) (`KismetMathLibrary.MakeRotator` 0.0 -10.0 (* (`KismetMathLibrary.DegSin` _output_get) 11.0)) false false))

(fn `UserConstructionScript`)